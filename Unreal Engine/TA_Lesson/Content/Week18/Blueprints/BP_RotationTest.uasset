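; BP_RotationTest is a test actor that spawns a ring of BP_ChairActor chairs around itself on BeginPlay.
; A loop uses cosine and sine of tenth-turn angle steps to place each chair on a fixed-radius horizontal circle.
; MakeRotFromX on the negated offset turns each chair to face the center.
; The inclusive loop bounds put the last spawn on top of the first.
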(event EventBeginPlay
  (for _index (range 0 10)
    (Game|SpawnActorfromClass "/Game/Week18/Blueprints/BP_ChairActor.BP_ChairActor_C" (Math|Transform|MakeTransform (+ (Transformation|GetActorLocation) (Math|Vector|MakeVector (* (Math|Trig|Cos(Radians) (* _index (/ (* (Math|Trig|GetPI) 2.0) 1e+01))) 5e+02) (* (Math|Trig|Sin(Radians) (* _index (/ (* (Math|Trig|GetPI) 2.0) 1e+01))) 5e+02) 0.0)) (Math|Rotator|MakeRotfromX (* (Math|Vector|MakeVector (* (Math|Trig|Cos(Radians) (* _index (/ (* (Math|Trig|GetPI) 2.0) 1e+01))) 5e+02) (* (Math|Trig|Sin(Radians) (* _index (/ (* (Math|Trig|GetPI) 2.0) 1e+01))) 5e+02) 0.0) -1.0)) "1.000000,1.000000,1.000000") "Undefined" "MultiplyWithRoot" 0 0)))

(fn ConstructionScript)