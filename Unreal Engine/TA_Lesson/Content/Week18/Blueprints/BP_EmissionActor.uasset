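; BP_EmissionActor is an actor that shows a randomly chosen static mesh with a configurable emissive color.
; Its construction script picks a mesh from the StaticMeshes array, applies Material, and writes EmissionColor, divided by 255, to the "Emission Color" parameter.
; An unconnected random HSV color branch remains, using a helper that remaps values from [-1,1] to [0.5,1].
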(fn ConstructionScript
  (bind _staticmeshes (Variables|Default|GetStaticMeshes))
  (bind _emission_color (Variables|Default|GetEmission%20Color))
  (Components|StaticMesh|SetStaticMesh (Variables|Default|GetStaticMesh) (Utilities|Array|Get(acopy) _staticmeshes (Math|Random|RandomIntegerinRange 0 (- (Utilities|Array|Length _staticmeshes) 1))))
  (Rendering|Material|SetMaterial (Variables|Default|GetStaticMesh) 0 (Variables|Default|GetMaterial))
  (Rendering|Material|SetColorParameterValueonMaterials (Variables|Default|GetStaticMesh) "Emission Color" (Utilities|Struct|MakeLinearColor (/ (.r _emission_color) 255.0) (/ (.g _emission_color) 255.0) (/ (.b _emission_color) 255.0) 1.0)))

(fn [-1,1]To[1/2,1]
  (params (In :type Float%20%28double-precision%29))
  (return (+ (* (/ (- In -1.0) 2.0) 0.5) 0.5)))