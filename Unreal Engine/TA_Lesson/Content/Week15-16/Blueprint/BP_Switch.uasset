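; BP_Switch is a physical push-button switch that fires its OnHitted event dispatcher when the Button component is hit.
; A hit disables the button's collision and plays the Press timeline, which drives the button's relative location.
; When Press finishes, the Bounce timeline plays from the start to move the button again, then restores collision so it can register another hit.
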(event OnComponentHit(Button)
  (params (HitComponent :type Primitive%20Component%20Object%20Reference) (OtherActor :type Actor%20Object%20Reference) (OtherComp :type Primitive%20Component%20Object%20Reference) (NormalImpulse :type Vector :default "0, 0, 0") (Hit :type Hit%20Result%20Structure%20%28by%20ref%29))
  (Default|CallOnHitted)
  (Collision|SetCollisionEnabled (Variables|Default|GetButton) "NoCollision")
  (bind _value (Timeline|Press Play)
    (:Update
      (Transformation|SetRelativeLocation (Variables|Default|GetButton) _value false false))
    (:Finished
      (bind _value_2 (Timeline|Bounce PlayFromStart)
        (:Update
          (Transformation|SetRelativeLocation (Variables|Default|GetButton) _value_2 false false))
        (:Finished
          (Collision|SetCollisionEnabled (Variables|Default|GetButton) "QueryAndPhysics"))))))

(fn ConstructionScript)