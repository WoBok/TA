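; BP_Stair is a stair actor that can be faded in and out through its Show and Hide events.
; Each event stops the opposite timeline, then plays its own from the start, driving the static mesh material's Alpha parameter.
; Show unhides the actor and restores collision immediately, while Hide waits for its fade to finish before hiding the actor and disabling collision.
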(event Custom|Show
  (Utilities|FlowControl|Sequence
    (:then_0
      (bind _value (Timeline|MaterialHide Stop)
        (:Update
          (Rendering|Material|SetScalarParameterValueonMaterials (Variables|Default|GetStaticMesh) "Alpha" _value))
        (:Finished
          (Rendering|SetActorHiddenInGame true)
          (Collision|SetCollisionEnabled (Variables|Default|GetStaticMesh) "NoCollision"))))
    (:then_1
      (Rendering|SetActorHiddenInGame false)
      (Collision|SetCollisionEnabled (Variables|Default|GetStaticMesh) "QueryAndPhysics")
      (bind _value_2 (Timeline|MaterialShow PlayFromStart)
        (:Update
          (Rendering|Material|SetScalarParameterValueonMaterials (Variables|Default|GetStaticMesh) "Alpha" _value_2))))))

(event Custom|Hide
  (Utilities|FlowControl|Sequence
    (:then_0
      (bind _value (Timeline|MaterialShow Stop)
        (:Update
          (Rendering|Material|SetScalarParameterValueonMaterials (Variables|Default|GetStaticMesh) "Alpha" _value))))
    (:then_1
      (bind _value_2 (Timeline|MaterialHide PlayFromStart)
        (:Update
          (Rendering|Material|SetScalarParameterValueonMaterials (Variables|Default|GetStaticMesh) "Alpha" _value_2))
        (:Finished
          (Rendering|SetActorHiddenInGame true)
          (Collision|SetCollisionEnabled (Variables|Default|GetStaticMesh) "NoCollision"))))))

(fn ConstructionScript)