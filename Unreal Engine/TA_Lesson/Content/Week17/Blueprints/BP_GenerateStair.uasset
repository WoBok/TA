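; Spawns a staircase of BP_Stair actors that appears and disappears step by step.
; On BeginPlay, transform helpers lay out a half-circle rising arc and a straight run that levels off, then hidden steps are spawned into one array.
; ShowOrHide toggles behind a busy flag: steps rise into place sequentially via a timeline, or hide in reverse with short delays.
; GenerateStair duplicates the layout logic but is not called here.
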(event Custom|ShowOrHide
  (if (!= (Variables|Default|GetIsShowingOrHiding) true)
    (Variables|Default|SetIsShowingOrHiding true)
    (if (Variables|Default|GetShowHide)
      (Variables|Default|SetStairIndex 0)
      (Default|Show (Utilities|Array|Get(acopy) (Variables|Default|GetStairs) (Variables|Default|GetStairIndex)) :!label _label)
      (Variables|Default|SetTargetPosition (Transformation|GetActorLocation (Utilities|Array|Get(acopy) (Variables|Default|GetStairs) (Variables|Default|GetStairIndex))))
      (Transformation|SetActorLocation (Utilities|Array|Get(acopy) (Variables|Default|GetStairs) (Variables|Default|GetStairIndex)) (- (Transformation|GetActorLocation (Utilities|Array|Get(acopy) (Variables|Default|GetStairs) (Variables|Default|GetStairIndex))) (Math|Vector|MakeVector 0.0 0.0 (* (Variables|Default|GetStepHeight) 3.0))) false false)
      (bind _lerp (Timeline|ZeroToOne PlayFromStart)
        (:Update
          (Transformation|SetActorLocation (Utilities|Array|Get(acopy) (Variables|Default|GetStairs) (Variables|Default|GetStairIndex)) (Math|Vector|Lerp(Vector) (Transformation|GetActorLocation (Utilities|Array|Get(acopy) (Variables|Default|GetStairs) (Variables|Default|GetStairIndex))) (Variables|Default|GetTargetPosition) _lerp) false false))
        (:Finished
          (Math|Integer|IncrementInt (Variables|Default|GetStairIndex)
            (:%20%20
              (if (< (Variables|Default|GetStairIndex) (Utilities|Array|Length (Variables|Default|GetStairs)))
                (goto _label)
                (else
                  (Variables|Default|SetShowHide false)
                  (Variables|Default|SetIsShowingOrHiding false)))))))
      (else
        (bind _output_get (Variables|Default|SetStairIndex (- (Utilities|Array|Length (Variables|Default|GetStairs)) 1)))
        (Default|Hide (Utilities|Array|Get(acopy) (Variables|Default|GetStairs) _output_get) :!label _label_2)
        (Utilities|FlowControl|Delay 0.05)
        (bind _result (Math|Integer|DecrementInt (Variables|Default|GetStairIndex))
          (:%20%20
            (if (>= _result 0)
              (goto _label_2)
              (else
                (Variables|Default|SetShowHide true)
                (Variables|Default|SetIsShowingOrHiding false)))))))))

(event EventBeginPlay
  (Variables|Default|SetSelfTrans (Transformation|GetActorTransform))
  (bind _transforms (CallFunction|GenerateFirstPosRot (Variables|Default|GetSelfTrans)))
  (bind _stairs (CallFunction|GenerateStariSteps _transforms))
  (Variables|Default|SetStairs _stairs)
  (bind _transforms_2 (CallFunction|GenerateSecondPosRot (Variables|Default|GetSelfTrans)))
  (bind _stairs_2 (CallFunction|GenerateStariSteps _transforms_2))
  (Utilities|Array|AppendArray (Variables|Default|GetStairs) _stairs_2))

(fn ConstructionScript)

(fn GenerateStair
  (bind _stepheight (Variables|Default|GetStepHeight))
  (LocalVariables|SetSelfTransform (Transformation|GetActorTransform))
  (for _index (range 0 (Variables|Default|GetFirstStairNum))
    (Game|SpawnActorfromClass "/Game/Week17/Blueprints/BP_Stair.BP_Stair_C" (Math|Transform|MakeTransform (+ (Math|Vector|MakeVector (* (Variables|Default|GetFirstStairRadius) (Math|Trig|Cos(Radians) (- (Math|Float|MultiplybyPi 1.0) (* _index (/ (Math|Float|MultiplybyPi 1.0) (Variables|Default|GetFirstStairNum)))))) (* (Variables|Default|GetFirstStairRadius) (Math|Trig|Sin(Radians) (- (Math|Float|MultiplybyPi 1.0) (* _index (/ (Math|Float|MultiplybyPi 1.0) (Variables|Default|GetFirstStairNum)))))) (* _index (Variables|Default|GetStepHeight))) (.location (LocalVariables|GetSelfTransform))) (Math|Rotator|MakeRotator (.roll (.rotation (LocalVariables|GetSelfTransform))) (.pitch (.rotation (LocalVariables|GetSelfTransform))) (Math|Trig|RadiansToDegrees (- (Math|Float|MultiplybyPi 1.0) (* _index (/ (Math|Float|MultiplybyPi 1.0) (Variables|Default|GetFirstStairNum)))))) (.scale (LocalVariables|GetSelfTransform))) "Undefined" "MultiplyWithRoot" 0 0))
  (LocalVariables|SetSecondStairPosStart (+ (.location (LocalVariables|GetSelfTransform)) (Math|Vector|MakeVector (Variables|Default|GetFirstStairRadius) 0.0 (* (Variables|Default|GetFirstStairNum) (Variables|Default|GetStepHeight)))))
  (for _index_2 (range 1 (+ (Variables|Default|GetFirstStairNum) -8))
    (Game|SpawnActorfromClass "/Game/Week17/Blueprints/BP_Stair.BP_Stair_C" (Math|Transform|MakeTransform (Math|Vector|MakeVector (.x (LocalVariables|GetSecondStairPosStart)) (- (.y (LocalVariables|GetSecondStairPosStart)) (* _index_2 (Variables|Default|GetSecondStairInterval))) (+ (.z (LocalVariables|GetSecondStairPosStart)) (Math|Float|SelectFloat (* _index_2 _stepheight) (* _stepheight 1e+01) (<= _index_2 10)))) "0, 0, 0" "1.000000,1.000000,1.000000") "Undefined" "MultiplyWithRoot" 0 0)))

(fn GenerateFirstPosRot
  (params (SelfTrans :type Transform))
  (for _index (range 0 (Variables|Default|GetFirstStairNum))
    (Utilities|Array|Add (LocalVariables|GetTransformsArray) (Math|Transform|MakeTransform (+ (Math|Vector|MakeVector (* (Variables|Default|GetFirstStairRadius) (Math|Trig|Cos(Radians) (- (Math|Float|MultiplybyPi 1.0) (* _index (/ (Math|Float|MultiplybyPi 1.0) (Variables|Default|GetFirstStairNum)))))) (* (Variables|Default|GetFirstStairRadius) (Math|Trig|Sin(Radians) (- (Math|Float|MultiplybyPi 1.0) (* _index (/ (Math|Float|MultiplybyPi 1.0) (Variables|Default|GetFirstStairNum)))))) (* _index (Variables|Default|GetStepHeight))) (.location SelfTrans)) (Math|Rotator|MakeRotator (.roll (.rotation SelfTrans)) (.pitch (.rotation SelfTrans)) (Math|Trig|RadiansToDegrees (- (Math|Float|MultiplybyPi 1.0) (* _index (/ (Math|Float|MultiplybyPi 1.0) (Variables|Default|GetFirstStairNum)))))))))
  (return (LocalVariables|GetTransformsArray)))

(fn GenerateSecondPosRot
  (params (SelfTrans :type Transform))
  (bind _stepheight (Variables|Default|GetStepHeight))
  (LocalVariables|SetStartPos (+ (.location SelfTrans) (Math|Vector|MakeVector (Variables|Default|GetFirstStairRadius) 0.0 (* (Variables|Default|GetFirstStairNum) (Variables|Default|GetStepHeight)))))
  (for _index (range 1 (Variables|Default|GetSecondStairNum))
    (Utilities|Array|Add (LocalVariables|GetTransformsArray) (Math|Transform|MakeTransform (Math|Vector|MakeVector (.x (LocalVariables|GetStartPos)) (- (.y (LocalVariables|GetStartPos)) (* _index (Variables|Default|GetSecondStairInterval))) (+ (.z (LocalVariables|GetStartPos)) (Math|Float|SelectFloat (* _index _stepheight) (* _stepheight 1e+01) (<= _index 10)))))))
  (return (LocalVariables|GetTransformsArray)))

(fn GenerateStariSteps
  (params (Treansforms :type Array%20of%20Transforms))
  (for _array_element Treansforms
    (bind _returnvalue (Game|SpawnActorfromClass "/Game/Week17/Blueprints/BP_Stair.BP_Stair_C" _array_element "Undefined" "MultiplyWithRoot" 0 0))
    (Rendering|SetActorHiddenInGame _returnvalue true)
    (Utilities|Array|Add (LocalVariables|GetStairsArray) _returnvalue))
  (return (LocalVariables|GetStairsArray)))