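; BP_Emission_Primitive is a mesh actor that sends out an emissive color wave from the point where a first-person projectile hits it.
; Each hit sets a random HSV color and the world-space impact point on the material, plays a sound, and restarts the progress timeline.
; When that finishes, it flags Revert and plays an inverse timeline.
; The construction script passes the scaled bounds diagonal to the material as Max Boundary.
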(event OnComponentHit(StaticMesh)
  (params (HitComponent :type Primitive%20Component%20Object%20Reference) (OtherActor :type Actor%20Object%20Reference) (OtherComp :type Primitive%20Component%20Object%20Reference) (NormalImpulse :type Vector :default "0, 0, 0") (Hit :type Hit%20Result%20Structure%20%28by%20ref%29))
  (bind _impactpoint (Collision|BreakHitResult Hit))
  (bind _returnvalue (Math|Random|RandomUnitVector))
  (Utilities|Casting|CastToBP_FirstPersonProjectile OtherActor)
  (Utilities|FlowControl|Sequence
    (:then_0
      (Rendering|Material|SetColorParameterValueonMaterials (Variables|Default|GetStaticMesh) "Emissive Color" (Class|KismetMathLibrary|HSVtoRGB (* (+ (* (.x _returnvalue) 0.5) 0.5) 365.0) (* (CallFunction|[-1,1]To[1/2,1] (.y _returnvalue)) 1e+01) (* (CallFunction|[-1,1]To[1/2,1] (.z _returnvalue)) 1e+01) 1.0)))
    (:then_1
      (Rendering|Material|SetVectorParameterValueonMaterials (Variables|Default|GetStaticMesh) "Hit PositionWS" _impactpoint)
      (Audio|PlaySoundatLocation "/Game/Week17/Audio/MS_LightWave.MS_LightWave" _impactpoint "0, 0, 0" 1.0 1.0 0.0 0 0 0 0))
    (:then_2
      (bind _emission_progress (Timeline|Emission%20Progress%20Invert Stop)
        (:Update
          (Rendering|Material|SetScalarParameterValueonMaterials (Variables|Default|GetStaticMesh) "Progress" _emission_progress))))
    (:then_3
      (Rendering|Material|SetScalarParameterValueonMaterials (Variables|Default|GetStaticMesh) "Revert" 0.0)
      (bind _emission_progress_2 (Timeline|Emission%20Progress PlayFromStart)
        (:Update
          (Rendering|Material|SetScalarParameterValueonMaterials (Variables|Default|GetStaticMesh) "Progress" _emission_progress_2))
        (:Finished
          (Rendering|Material|SetScalarParameterValueonMaterials (Variables|Default|GetStaticMesh) "Revert" 1.0)
          (Timeline|Emission%20Progress%20Invert PlayFromStart))))))

(fn ConstructionScript
  (bind _staticmesh (Variables|Default|GetStaticMesh))
  (bind _staticmesh_2 (Variables|Default|GetStaticMesh))
  (bind (_min _max) (Components|StaticMesh|GetLocalBounds _staticmesh))
  (bind _returnvalue (Transformation|GetWorldScale _staticmesh_2))
  (bind _returnvalue_2 (- _max _min))
  (bind _returnvalue_3 (* _returnvalue_2 _returnvalue))
  (Rendering|Material|SetScalarParameterValueonMaterials (Variables|Default|GetStaticMesh) "Max Boundary" (Math|Float|Sqrt (Math|Vector|DotProduct _returnvalue_3 _returnvalue_3))))

(fn [-1,1]To[1/2,1]
  (params (In :type Float%20%28double-precision%29))
  (return (+ (* (/ (- In -1.0) 2.0) 0.5) 0.5)))