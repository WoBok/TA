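; BP_RefrectionItem is a mesh actor that feeds a random base color and the player's location into its materials, apparently for a refraction effect.
; The construction script builds the color in HSV from random unit vector components, using a helper that remaps [-1,1] to [0.5,1] before saturation and value are scaled up.
; Every tick it writes the first player character's location to the PlayerPosition material parameter.
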(event EventTick
  (params (DeltaSeconds :type Float%20%28single-precision%29))
  (Rendering|Material|SetVectorParameterValueonMaterials (Variables|Default|GetStaticMesh) "PlayerPosition" (Transformation|GetActorLocation (Game|GetPlayerCharacter 0))))

(fn ConstructionScript
  (bind _returnvalue (Math|Random|RandomUnitVector))
  (Rendering|Material|SetColorParameterValueonMaterials (Variables|Default|GetStaticMesh) "Base Color" (Class|KismetMathLibrary|HSVtoRGB (* (+ (* (.x _returnvalue) 0.5) 0.5) 365.0) (* (CallFunction|[-1,1]To[1/2,1] (.y _returnvalue)) 1e+01) (* (CallFunction|[-1,1]To[1/2,1] (.z _returnvalue)) 1e+01) 1.0)))

(fn [-1,1]To[1/2,1]
  (params (In :type Float%20%28double-precision%29))
  (return (+ (* (/ (- In -1.0) 2.0) 0.5) 0.5)))